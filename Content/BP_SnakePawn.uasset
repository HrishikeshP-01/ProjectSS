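; BP_SnakePawn is a player-controlled, physics-driven snake with a head-mounted camera boom.
; It generates a chain of tapering spheres joined by physics constraints, rebuilding a spline through them each tick to deform head, body and tail spline meshes.
; Input pushes only the head sphere for steering, timed upward thrust, descent and strikes, with trigger boost scaled by body curvature.
; E toggles a debug-shape view of the chain.
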(event `self.ReceiveBeginPlay`
  (bind _springarm (`self.SpringArm`))
  ;[1 0.6642 0] Begin Play
  (`|ExecutionSequence`
    (:`then_0`
      (if (or (not (`self.Create Via Construction Script`)) (`self.Force Creation On Begin Play`))
        (`self.Add Collision Spheres`)
        (`self.Add Spline Meshes`)))
    (:`then_1`
      (`self.Add Physics Constraints`)
      (`self.Add Spline Component`))
    (:`then_2`
      (bind _return_value (`self.Get Head Collision Shape`))
      (`SceneComponent.K2_AttachToComponent` _springarm _return_value "None" "SnapToTarget" "SnapToTarget" "SnapToTarget" true)
      (set `SpringArmComponent.bUsePawnControlRotation` true _springarm))))

(event `InputAxis|TurnRate`
  (params (AxisValue :type "Float (single-precision)"))
  ;[1 1 1] Input
  (`self.AddControllerYawInput` (* AxisValue (`self.Base Turn Rate`) (`GameplayStatics.GetWorldDeltaSeconds`))))

(event `Key|E`
  (params (Key :type "Key Structure"))
  ;[0 0.3291 0.48] Tick
  (:`Pressed`
    (`/Engine/EditorBlueprintResources/StandardMacros.FlipFlop`
      (:`A`
        (`self.Set Snake Mesh Visibility` false)
        (goto _label :!via `Open`))
      (:`B`
        (`self.Set Snake Mesh Visibility` true)
        (goto _label :!via `Close`)))))

(event `self.ReceiveTick`
  (params (DeltaSeconds :type "Float (single-precision)"))
  (bind _returnvalue (- (`SplineComponent.GetNumberOfSplinePoints` (`self.Spline Component`)) 2))
  ;[0 0.3291 0.48] Tick
  (`|ExecutionSequence`
    (:`then_0`
      (`self.Update Spline Component`)
      (`self.Update Snake Mesh`)
      (`/Engine/EditorBlueprintResources/StandardMacros.Gate` true :!label _label
        (:`Exit`
          (`self.Draw Debug Shapes`))))
    (:`then_2`
      (set `self.Current Strech Ratio` 0.0)
      (for _index (range 2 (+ _returnvalue 1))
        (set `self.Current Strech Ratio` (+ (`KismetMathLibrary.Lerp` 0.2 4.0 (- 1.0 (`KismetMathLibrary.Abs` (`KismetMathLibrary.Dot_VectorVector` (`KismetMathLibrary.Normal` (`SplineComponent.GetTangentAtSplinePoint` (`self.Spline Component`) _index "Local")) (`KismetMathLibrary.Normal` (`SplineComponent.GetTangentAtSplinePoint` (`self.Spline Component`) (+ _index 1) "Local")))))) (`self.Current Strech Ratio`))))
      (set `self.Current Strech Ratio` (`KismetMathLibrary.FClamp` (/ (`self.Current Strech Ratio`) (`KismetMathLibrary.Conv_IntToDouble` _returnvalue)) 0.0 0.5)))
    (:`then_3`
      (`SceneComponent.K2_SetWorldLocation` (`self.DefaultSceneRoot`) (`SceneComponent.K2_GetComponentLocation` (`self.SpringArm`)) false false))))

(event `InputAxis|LookUpRate`
  (params (AxisValue :type "Float (single-precision)"))
  ;[1 1 1] Input
  (`self.AddControllerPitchInput` (* AxisValue (`self.Base Look Up Rate`) (`GameplayStatics.GetWorldDeltaSeconds`))))

(event `InputAxis|Turn` :overrideparent false
  (params (AxisValue :type "Float (single-precision)"))
  ;[1 1 1] Input
  (`self.AddControllerYawInput` AxisValue))

(event `InputAxis|LookUp` :overrideparent false
  (params (AxisValue :type "Float (single-precision)"))
  ;[1 1 1] Input
  (`self.AddControllerPitchInput` AxisValue))

(event `InputAxis|MoveUp`
  (params (AxisValue :type "Float (single-precision)"))
  ;[0.6567 1 0.5724] Debug
)

(event `InputAction|UpwardThrust`
  (params (Key :type "Key Structure"))
  ;[1 1 1] Input
  (:`Pressed`
    (bind (_direction _thrustmultiplier _staminapercent) (`Timeline|Timeline_0` :!label _label_2)
      (:`Update`
        (bind _return_value (`self.Get Head Collision Shape`))
        (`PrimitiveComponent.AddImpulse` _return_value (* (0.0 0.0 1.0) (* _thrustmultiplier (`self.Move Up Impulse`))) "None" true)
        (set `self.Stamina` _staminapercent))
      (:`Finished`
        (goto _label_2 :!via `SetNewTime`))))
  (:`Released`
    (`|ExecutionSequence`
      (:`then_0`
        (goto _label_2 :!via `Stop`))
      (:`then_1`
        (`KismetSystemLibrary.Delay` 0.5)
        (set `self.Stamina` 1.0)
        (goto _label_2 :!via `SetNewTime`)))))

(event `InputAxis|MoveDown`
  (params (AxisValue :type "Float (single-precision)"))
  ;[1 1 1] Input
  (bind _return_value (`self.Get Head Collision Shape`))
  (`PrimitiveComponent.AddImpulse` _return_value (* (0.0 0.0 1.0) (* AxisValue (`self.Move Down Impulse`) -1.0)) "None" true))

(event `Update Spline Component`
  (bind _collision_spheres_list (`self.Collision Spheres List`))
  ;[1 0.05914 0] Custom Evnets
  (`SplineComponent.ClearSplinePoints` (`self.Spline Component`) false)
  (for (_array_element _array_index) _collision_spheres_list
    (`SplineComponent.AddSplinePoint` (`self.Spline Component`) (`SceneComponent.K2_GetComponentLocation` _array_element) "World" (== _array_index (`KismetArrayLibrary.Array_LastIndex` _collision_spheres_list)))))

(event `InputAxis|MoveForward`
  (params (AxisValue :type "Float (single-precision)"))
  (bind _move_forward_power (`self.Move Forward Power`))
  (bind _current_right_trigger_axis (`self.Current Right Trigger Axis`))
  ;[1 1 1] Input
  (bind _return_value (`self.Get Head Collision Shape`))
  (`PrimitiveComponent.AddForce` _return_value (* (`KismetMathLibrary.Normal` (`KismetMathLibrary.ProjectVectorOnToPlane` (`SceneComponent.GetForwardVector` (`self.Camera`)) (0.0 0.0 1.0))) (select `bool` (> _current_right_trigger_axis 0.05) :`false` (* AxisValue _move_forward_power) :`true` (+ _move_forward_power (* (`self.Speed Boost Power`) (`self.Current Strech Ratio`) _current_right_trigger_axis)))) "None" true))

(event `Update Snake Mesh`
  ;[1 0.05914 0] Custom Evnets
  (for (_array_element _array_index) (`self.Spline Meshes List`)
    (bind (_location _tangent) (`SplineComponent.GetLocationAndTangentAtSplinePoint` (`self.Spline Component`) _array_index "Local"))
    (bind _returnvalue (+ _array_index 1))
    (bind (_location_2 _tangent_2) (`SplineComponent.GetLocationAndTangentAtSplinePoint` (`self.Spline Component`) _returnvalue "Local"))
    (`SplineMeshComponent.SetStartAndEnd` _array_element (- _location (* (`KismetMathLibrary.Normal` _tangent) (`SphereComponent.GetScaledSphereRadius` (`|GetArrayItem` (`self.Collision Spheres List`) _array_index)))) _tangent (- _location_2 (* (`KismetMathLibrary.Normal` _tangent_2) (`SphereComponent.GetScaledSphereRadius` (`|GetArrayItem` (`self.Collision Spheres List`) _returnvalue)))) _tangent_2 false)
    (`SplineMeshComponent.SetSplineUpDir` _array_element (`SplineComponent.GetUpVectorAtSplinePoint` (`self.Spline Component`) _array_index "Local") true)))

(event `InputAxisKey|Gamepad_RightTriggerAxis`
  (params (AxisValue :type "Float (single-precision)"))
  ;[1 1 1] Input
  (set `self.Current Right Trigger Axis` AxisValue))

(event `InputAxis|MoveRight`
  (params (AxisValue :type "Float (single-precision)"))
  ;[1 1 1] Input
  (bind _return_value (`self.Get Head Collision Shape`))
  (`PrimitiveComponent.AddForce` _return_value (* (`KismetMathLibrary.Normal` (`KismetMathLibrary.ProjectVectorOnToPlane` (`SceneComponent.GetRightVector` (`self.Camera`)) (0.0 0.0 1.0))) (* (`self.Move Right Power`) AxisValue)) "None" true))

(event `Set Snake Mesh Visibility`
  (params (bNewVisibility :type Boolean))
  ;[1 0.05914 0] Custom Evnets
  (for _array_element (`self.Spline Meshes List`)
    (`/Engine/EditorBlueprintResources/StandardMacros.IsValid` _array_element
      (:`Is Valid`
        (`SceneComponent.SetVisibility` _array_element bNewVisibility false)))))

(event `InputAction|Strike`
  (params (Key :type "Key Structure"))
  (:`Pressed`
    (set `self.IsBiting` true)
    (bind _return_value (`self.Get Head Collision Shape`))
    (`PrimitiveComponent.AddImpulse` _return_value (* (`SceneComponent.GetForwardVector` (`self.Camera`)) 2000.0) "None" true))
  (:`Released`
    (set `self.IsBiting` false)))

(event `Draw Debug Shapes`
  (bind (_location _tangent) (`SplineComponent.GetLocationAndTangentAtSplinePoint` (`self.Spline Component`) 0 "World"))
  ;[1 0.05914 0] Custom Evnets
  (for (_array_element _array_index) (`self.Collision Spheres List`)
    (`KismetSystemLibrary.DrawDebugSphere` (`SceneComponent.K2_GetComponentLocation` _array_element) (`SphereComponent.SphereRadius` _array_element) 16 (`self.Debug Sphere Color`))
    (if (< _array_index (- (`KismetArrayLibrary.Array_Length` (`self.Collision Spheres List`)) 1))
      (bind _output (`|GetArrayItem` (`self.Collision Spheres List`) _array_index))
      (`KismetSystemLibrary.DrawDebugLine` (`SceneComponent.K2_GetComponentLocation` _output) (`SceneComponent.K2_GetComponentLocation` (`|GetArrayItem` (`self.Collision Spheres List`) (+ _array_index 1))) (`self.Debug Line Color`) 0.0 (* (`SphereComponent.SphereRadius` _output) 2.0 (`self.Debug Line Scale`)))))
  (`KismetSystemLibrary.DrawDebugArrow` _location (+ _location (* (`KismetMathLibrary.Normal` _tangent) -50.0)) 20.0 (`self.Debug Line Color`) 0.0 5.0))

(fn `Add Collision Spheres`
  (returns (`Return Value` :type Boolean))
  (locals (TempIndex :type Integer) (TempRadius :type "Float (double-precision)") (TempDistance :type "Float (double-precision)"))
  (bind _default_radius (`self.Default Radius`))
  (bind _tempradius (`local.TempRadius`))
  (bind _collision_spheres_list (`self.Collision Spheres List`))
  (bind _returnvalue (`KismetArrayLibrary.Array_Length` (`self.Collision Spheres List`)))
  (bind _returnvalue_2 (* (`self.Nodes Count`) (`self.Scaling Down Start Ratio`)))
  (`|ExecutionSequence`
    (:`then_0`
      (if (!= (`KismetArrayLibrary.Array_Length` (`self.Collision Spheres List`)) 0)
        (for _array_element _collision_spheres_list
          (`/Engine/EditorBlueprintResources/StandardMacros.IsValid` _array_element
            (:`Is Valid`
              (`ActorComponent.K2_DestroyComponent` _array_element))))
        (`KismetArrayLibrary.Array_Clear` _collision_spheres_list)))
    (:`then_1`
      (for _index (range (`self.Nodes Count`))
        (set `local.TempIndex` _index)
        (set `local.TempRadius` (select `bool` (< _returnvalue_2 (`KismetMathLibrary.Conv_IntToDouble` (`local.TempIndex`))) :`false` (`self.Default Radius`) :`true` (`KismetMathLibrary.FMax` (`KismetMathLibrary.Lerp` _default_radius (* _default_radius (`self.Last Sphere Radius Ratio`)) (`KismetMathLibrary.FClamp` (/ (- (`KismetMathLibrary.Conv_IntToDouble` (`local.TempIndex`)) _returnvalue_2) (* (`self.Nodes Count`) (- 1.0 (`self.Scaling Down Start Ratio`)))))) 0.01)))
        (bind _returnvalue_3 (`AddComponent|NODE_AddSphereComponent-1` :`RelativeTransform` (`KismetMathLibrary.MakeTransform` (`KismetMathLibrary.MakeVector` (`local.TempDistance`)))))
        (`SphereComponent.SetSphereRadius` _returnvalue_3 (`local.TempRadius`) true)
        (set `local.TempDistance` (+ (`local.TempDistance`) _tempradius _tempradius (`self.Extra Spacing`)))
        (`PrimitiveComponent.SetMassOverrideInKg` _returnvalue_3 "None" (* (/ (`local.TempRadius`) (`self.Default Radius`)) (`self.Default Mass`) (select `bool` (== (`local.TempIndex`) 0) :`false` 1.0 :`true` (`self.Head Mass Scale`))) true)
        (`PrimitiveComponent.SetLinearDamping` _returnvalue_3 (`self.Linear Damping`))
        (`PrimitiveComponent.SetAngularDamping` _returnvalue_3 (`self.Angular Damping`))
        (`PrimitiveComponent.SetPhysMaterialOverride` _returnvalue_3 (`self.Physical Material`))
        (`KismetArrayLibrary.Array_Add` (`self.Collision Spheres List`) _returnvalue_3)))
    (:`then_2`
      (return (and (!= _returnvalue 0) (== _returnvalue (`self.Nodes Count`)))))))

(fn `Add Physics Constraints`
  (returns (`Return Value` :type Boolean))
  (bind _collision_spheres_list (`self.Collision Spheres List`))
  (if (> (`KismetArrayLibrary.Array_Length` (`self.Collision Spheres List`)) 0)
    (`|ExecutionSequence`
      (:`then_0`
        (for (_array_element _array_index) _collision_spheres_list
          (if (< _array_index (- (`KismetArrayLibrary.Array_Length` _collision_spheres_list) 1))
            (bind _returnvalue (`AddComponent|NODE_AddPhysicsConstraintComponent-1`))
            (bind _output (`|GetArrayItem` (`self.Collision Spheres List`) (+ _array_index 1)))
            (`SceneComponent.K2_SetWorldLocation` _returnvalue (/ (+ (`SceneComponent.K2_GetComponentLocation` _array_element) (`SceneComponent.K2_GetComponentLocation` _output)) 2.0) false false)
            (`PhysicsConstraintComponent.SetConstrainedComponents` _returnvalue _output "None" _array_element "None")
            (`KismetArrayLibrary.Array_Add` (`self.Physics Constraints List`) _returnvalue))))
      (:`then_1`
        (return (== (`KismetArrayLibrary.Array_Length` (`self.Physics Constraints List`)) (- (`self.Nodes Count`) 1)))))
    (else
      (return false))))

(fn `Add Spline Component`
  (bind _returnvalue (`AddComponent|NODE_AddSplineComponent-0` :`RelativeTransform` (`KismetMathLibrary.MakeTransform` (0.0 0.0 0.0))))
  (bind _output_get (set `self.Spline Component` _returnvalue))
  (`SceneComponent.SetAbsolute` _output_get true true true)
  (`SplineComponent.ClearSplinePoints` (`self.Spline Component`) true))

(fn `Add Spline Meshes`
  (returns (`Return Value` :type Boolean))
  (locals (`Temp Index` :type Integer))
  (bind _returnvalue (`self.GetActorForwardVector`))
  (bind _collision_spheres_list (`self.Collision Spheres List`))
  (bind _spline_meshes_list (`self.Spline Meshes List`))
  (if (> (`KismetArrayLibrary.Array_Length` (`self.Collision Spheres List`)) 0)
    (`|ExecutionSequence`
      (:`then_0`
        (if (!= (`KismetArrayLibrary.Array_Length` (`self.Spline Meshes List`)) 0)
          (for _array_element _spline_meshes_list
            (`/Engine/EditorBlueprintResources/StandardMacros.IsValid` _array_element
              (:`Is Valid`
                (`ActorComponent.K2_DestroyComponent` _array_element))))
          (`KismetArrayLibrary.Array_Clear` _spline_meshes_list)))
      (:`then_1`
        (for (_array_element_2 _array_index) _collision_spheres_list
          (bind _output_get (set `local.Temp Index` _array_index))
          (if (< _output_get (- (`KismetArrayLibrary.Array_Length` _collision_spheres_list) 1))
            (bind _returnvalue_2 (`AddComponent|NODE_AddSplineMeshComponent-1` :`bManualAttachment` true))
            (`KismetArrayLibrary.Array_Add` (`self.Spline Meshes List`) _returnvalue_2)
            (bind _returnvalue_3 (/ (`SphereComponent.SphereRadius` _array_element_2) 50.0))
            (`SplineMeshComponent.SetStartScale` _returnvalue_2 (`KismetMathLibrary.MakeVector2D` _returnvalue_3 _returnvalue_3) true)
            (bind _output (`|GetArrayItem` (`self.Collision Spheres List`) (+ _array_index 1)))
            (bind _returnvalue_4 (/ (`SphereComponent.SphereRadius` _output) 50.0))
            (`SplineMeshComponent.SetEndScale` _returnvalue_2 (`KismetMathLibrary.MakeVector2D` _returnvalue_4 _returnvalue_4) true)
            (`SplineMeshComponent.SetStartAndEnd` _returnvalue_2 (`SceneComponent.K2_GetComponentLocation` _array_element_2) _returnvalue (`SceneComponent.K2_GetComponentLocation` _output) _returnvalue true)
            (`StaticMeshComponent.SetStaticMesh` _returnvalue_2 (select `bool` (== (`local.Temp Index`) (- (`self.Nodes Count`) 2)) :`false` (select `bool` (== (`local.Temp Index`) 0) :`false` (`self.Body Mesh`) :`true` (`self.Head Mesh`)) :`true` (`self.Tail Mesh`)))
            (if (and (> (`KismetArrayLibrary.Array_Length` (`self.Body Materials List`)) 0) (> (`local.Temp Index`) 0) (< (`local.Temp Index`) (- (`self.Nodes Count`) 2)))
              (`PrimitiveComponent.SetMaterial` _returnvalue_2 0 "/Game/Meshes/SnakeHead/snakeMat.snakeMat")))))
      (:`then_2`
        (return (== (`KismetArrayLibrary.Array_Length` (`self.Spline Meshes List`)) (- (`self.Nodes Count`) 1)))))
    (else
      (return false))))

(fn `Clear If Needed`
  (bind _collision_spheres_list (`self.Collision Spheres List`))
  (bind _spline_meshes_list (`self.Spline Meshes List`))
  (bind _physics_constraints_list (`self.Physics Constraints List`))
  (`|ExecutionSequence`
    (:`then_0`
      (for _array_element _collision_spheres_list
        (`/Engine/EditorBlueprintResources/StandardMacros.IsValid` _array_element
          (:`Is Valid`
            (`ActorComponent.K2_DestroyComponent` _array_element))))
      (`KismetArrayLibrary.Array_Clear` _collision_spheres_list))
    (:`then_1`
      (for _array_element_2 _spline_meshes_list
        (`/Engine/EditorBlueprintResources/StandardMacros.IsValid` _array_element_2
          (:`Is Valid`
            (`ActorComponent.K2_DestroyComponent` _array_element_2))))
      (`KismetArrayLibrary.Array_Clear` _spline_meshes_list))
    (:`then_2`
      (for _array_element_3 _physics_constraints_list
        (`/Engine/EditorBlueprintResources/StandardMacros.IsValid` _array_element_3
          (:`Is Valid`
            (`ActorComponent.K2_DestroyComponent` _array_element_3))))
      (`KismetArrayLibrary.Array_Clear` _physics_constraints_list))))

(fn `Get Head Collision Shape`
  (returns (`Return Value` :type "SphereComponent Object Reference"))
  (return (`|GetArrayItem` (`self.Collision Spheres List`))))

(fn `UserConstructionScript`
  (if (`self.Create Via Construction Script`)
    (`self.Add Collision Spheres`)
    (`self.Add Spline Meshes`)
    (else
      (`self.Clear If Needed`))))